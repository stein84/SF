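; Magic effect Blueprint for cards, with configurable color and brightness for its card, dust and ring elements.
; On BeginPlay it creates dynamic material instances for nine element indices and sets their "br" and "color" parameters.
; The first four take the Card variables, the next four the Dust variables and the last the Ring variables.
; Nothing updates afterward, as Tick, overlap and the construction script are empty.
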(event EventBeginPlay
  (bind _color_card (Variables|Default|Getcolor_card))
  (bind _color_dust (Variables|Default|Getcolor_dust))
  (bind _brightness_card (Variables|Default|Getbrightness_card))
  (bind _brightness_dust (Variables|Default|Getbrightness_dust))
  (bind _returnvalue (Rendering|Material|CreateDynamicMaterialInstance 0 0 :!class /Script/Engine.PrimitiveComponent))
  (Rendering|Material|SetScalarParameterValue _returnvalue "br" _brightness_card :!class /Script/Engine.MaterialInstanceDynamic)
  (Rendering|Material|SetVectorParameterValue _returnvalue "color" _color_card :!class /Script/Engine.MaterialInstanceDynamic)
  (bind _returnvalue_2 (Rendering|Material|CreateDynamicMaterialInstance 1 0 :!class /Script/Engine.PrimitiveComponent))
  (Rendering|Material|SetScalarParameterValue _returnvalue_2 "br" _brightness_card :!class /Script/Engine.MaterialInstanceDynamic)
  (Rendering|Material|SetVectorParameterValue _returnvalue_2 "color" _color_card :!class /Script/Engine.MaterialInstanceDynamic)
  (bind _returnvalue_3 (Rendering|Material|CreateDynamicMaterialInstance 2 0 :!class /Script/Engine.PrimitiveComponent))
  (Rendering|Material|SetScalarParameterValue _returnvalue_3 "br" _brightness_card :!class /Script/Engine.MaterialInstanceDynamic)
  (Rendering|Material|SetVectorParameterValue _returnvalue_3 "color" _color_card :!class /Script/Engine.MaterialInstanceDynamic)
  (bind _returnvalue_4 (Rendering|Material|CreateDynamicMaterialInstance 3 0 :!class /Script/Engine.PrimitiveComponent))
  (Rendering|Material|SetScalarParameterValue _returnvalue_4 "br" _brightness_card :!class /Script/Engine.MaterialInstanceDynamic)
  (Rendering|Material|SetVectorParameterValue _returnvalue_4 "color" _color_card :!class /Script/Engine.MaterialInstanceDynamic)
  (bind _returnvalue_5 (Rendering|Material|CreateDynamicMaterialInstance 4 0 :!class /Script/Engine.PrimitiveComponent))
  (Rendering|Material|SetScalarParameterValue _returnvalue_5 "br" _brightness_dust :!class /Script/Engine.MaterialInstanceDynamic)
  (Rendering|Material|SetVectorParameterValue _returnvalue_5 "color" _color_dust :!class /Script/Engine.MaterialInstanceDynamic)
  (bind _returnvalue_6 (Rendering|Material|CreateDynamicMaterialInstance 5 0 :!class /Script/Engine.PrimitiveComponent))
  (Rendering|Material|SetScalarParameterValue _returnvalue_6 "br" _brightness_dust :!class /Script/Engine.MaterialInstanceDynamic)
  (Rendering|Material|SetVectorParameterValue _returnvalue_6 "color" _color_dust :!class /Script/Engine.MaterialInstanceDynamic)
  (bind _returnvalue_7 (Rendering|Material|CreateDynamicMaterialInstance 6 0 :!class /Script/Engine.PrimitiveComponent))
  (Rendering|Material|SetScalarParameterValue _returnvalue_7 "br" _brightness_dust :!class /Script/Engine.MaterialInstanceDynamic)
  (Rendering|Material|SetVectorParameterValue _returnvalue_7 "color" _color_dust :!class /Script/Engine.MaterialInstanceDynamic)
  (bind _returnvalue_8 (Rendering|Material|CreateDynamicMaterialInstance 7 0 :!class /Script/Engine.PrimitiveComponent))
  (Rendering|Material|SetScalarParameterValue _returnvalue_8 "br" _brightness_dust :!class /Script/Engine.MaterialInstanceDynamic)
  (Rendering|Material|SetVectorParameterValue _returnvalue_8 "color" _color_dust :!class /Script/Engine.MaterialInstanceDynamic)
  (bind _returnvalue_9 (Rendering|Material|CreateDynamicMaterialInstance 8 0 :!class /Script/Engine.PrimitiveComponent))
  (Rendering|Material|SetScalarParameterValue _returnvalue_9 "br" (Variables|Default|Getbrightness_ring) :!class /Script/Engine.MaterialInstanceDynamic)
  (Rendering|Material|SetVectorParameterValue _returnvalue_9 "color" (Variables|Default|Getcolor_ring) :!class /Script/Engine.MaterialInstanceDynamic))

(event EventActorBeginOverlap
  (params (OtherActor :type Actor%20Object%20Reference)))

(event EventTick
  (params (DeltaSeconds :type Float%20%28single-precision%29)))

(fn ConstructionScript)