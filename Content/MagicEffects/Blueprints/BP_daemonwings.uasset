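; BP_daemonwings is a magic effect actor for demon wings with configurable color and brightness per layer: wings, cloud, dust and wave.
; BeginPlay creates dynamic material instances for six element slots and pushes those variables into their "br" and "color" parameters, with wings and wave covering two slots each.
; Tick runs through a short Delay into a non-resetting Activate, so activation is re-requested repeatedly while the actor lives.
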(event EventTick
  (params (DeltaSeconds :type Float%20%28single-precision%29))
  (Utilities|FlowControl|Delay 0.2)
  (Components|Activation|Activate false))

(event EventBeginPlay
  (bind _color_wings (Variables|Default|Getcolor_wings))
  (bind _color_wave (Variables|Default|Getcolor_wave))
  (bind _brightness_wings (Variables|Default|Getbrightness_wings))
  (bind _brightness_wave (Variables|Default|Getbrightness_wave))
  (bind _returnvalue (Rendering|Material|CreateDynamicMaterialInstance 0 0 :!class /Script/Engine.PrimitiveComponent))
  (Rendering|Material|SetScalarParameterValue _returnvalue "br" _brightness_wings :!class /Script/Engine.MaterialInstanceDynamic)
  (Rendering|Material|SetVectorParameterValue _returnvalue "color" _color_wings :!class /Script/Engine.MaterialInstanceDynamic)
  (bind _returnvalue_2 (Rendering|Material|CreateDynamicMaterialInstance 1 0 :!class /Script/Engine.PrimitiveComponent))
  (Rendering|Material|SetScalarParameterValue _returnvalue_2 "br" _brightness_wings :!class /Script/Engine.MaterialInstanceDynamic)
  (Rendering|Material|SetVectorParameterValue _returnvalue_2 "color" _color_wings :!class /Script/Engine.MaterialInstanceDynamic)
  (bind _returnvalue_3 (Rendering|Material|CreateDynamicMaterialInstance 2 0 :!class /Script/Engine.PrimitiveComponent))
  (Rendering|Material|SetScalarParameterValue _returnvalue_3 "br" (Variables|Default|Getbrightness_cloud) :!class /Script/Engine.MaterialInstanceDynamic)
  (Rendering|Material|SetVectorParameterValue _returnvalue_3 "color" (Variables|Default|Getcolor_cloud) :!class /Script/Engine.MaterialInstanceDynamic)
  (bind _returnvalue_4 (Rendering|Material|CreateDynamicMaterialInstance 3 0 :!class /Script/Engine.PrimitiveComponent))
  (Rendering|Material|SetScalarParameterValue _returnvalue_4 "br" (Variables|Default|Getbrightness_dust) :!class /Script/Engine.MaterialInstanceDynamic)
  (Rendering|Material|SetVectorParameterValue _returnvalue_4 "color" (Variables|Default|Getcolor_dust) :!class /Script/Engine.MaterialInstanceDynamic)
  (bind _returnvalue_5 (Rendering|Material|CreateDynamicMaterialInstance 4 0 :!class /Script/Engine.PrimitiveComponent))
  (Rendering|Material|SetScalarParameterValue _returnvalue_5 "br" _brightness_wave :!class /Script/Engine.MaterialInstanceDynamic)
  (Rendering|Material|SetVectorParameterValue _returnvalue_5 "color" _color_wave :!class /Script/Engine.MaterialInstanceDynamic)
  (bind _returnvalue_6 (Rendering|Material|CreateDynamicMaterialInstance 5 0 :!class /Script/Engine.PrimitiveComponent))
  (Rendering|Material|SetScalarParameterValue _returnvalue_6 "br" _brightness_wave :!class /Script/Engine.MaterialInstanceDynamic)
  (Rendering|Material|SetVectorParameterValue _returnvalue_6 "color" _color_wave :!class /Script/Engine.MaterialInstanceDynamic))

(event EventActorBeginOverlap
  (params (OtherActor :type Actor%20Object%20Reference)))

(fn ConstructionScript)